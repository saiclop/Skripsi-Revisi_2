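; BP_Player is a grid-based character that moves cell by cell and turns in 90-degree steps, tracking its grid coordinate and facing direction.
; MoveForward steps the coordinate along the facing direction and uses AI MoveTo to reach that cell's center, flagging movement until success.
; Turns update the direction and share a timeline that smoothly interpolates rotation.
; ResetPosition restores spawn cell and facing, while ResetPosition and Die sync the death flag to ABP_Character.
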(event `self.ReceiveBeginPlay`
  (bind _asbp_default_character (cast `/Game/Skripsi/Blueprints/BP_DefaultCharacter` (`GameplayStatics.GetPlayerCharacter` 0)))
  (set `self.Default Character` _asbp_default_character))

(event `MoveForward`
  (params (cells :type "Array of /Game/Skripsi/Blueprints/Maze/BP_Cell Object Reference") (size :type "IntPoint Structure") (gridSize :type Integer))
  (bind (_location_x _location_y) (break `IntPoint` (`self.location`)))
  (bind _returnvalue (`KismetMathLibrary.Conv_IntToDouble` (/ gridSize 2)))
  (set `self.move` true)
  (switch `EDirection` (`self.direction`)
    (:`Up`
      (set `self.location` (make `IntPoint` _location_x (- _location_y 1))))
    (:`Right`
      (set `self.location` (make `IntPoint` (+ _location_x 1) _location_y)))
    (:`Down`
      (set `self.location` (make `IntPoint` _location_x (+ _location_y 1))))
    (:`Left`
      (set `self.location` (make `IntPoint` (- _location_x 1) _location_y))))
  (`|AIMoveTo` self (+ (`self.K2_GetActorLocation` (`|GetArrayItem` cells (`/Game/Skripsi/Blueprints/F_Lib.GetIndex` (`self.location`) size))) (`KismetMathLibrary.MakeVector` _returnvalue _returnvalue)) null
    (:`OnSuccess`
      (set `self.move` false))))

(event `TurnRight`
  (bind _returnvalue (`self.K2_GetActorRotation`))
  (set `self.rotate` true)
  (set `self.currentRotation` _returnvalue)
  (set `self.nextRotation` (`KismetMathLibrary.ComposeRotators` _returnvalue (struct :`Yaw` 90.0)))
  (switch `EDirection` (`self.direction`)
    (:`Up`
      (set `self.direction` "Right")
      (bind (_direction _alpha) (`Timeline|RotationTimeline` :!via `PlayFromStart` :!label _label)
        (:`Update`
          (`self.K2_SetActorRotation` (`KismetMathLibrary.RLerp` (`self.currentRotation`) (`self.nextRotation`) _alpha true)))
        (:`Finished`
          (`self.K2_SetActorRotation` (`self.nextRotation`))
          (set `self.rotate` false))))
    (:`Right`
      (set `self.direction` "Down")
      (goto _label :!via `PlayFromStart`))
    (:`Down`
      (set `self.direction` "Left")
      (goto _label :!via `PlayFromStart`))
    (:`Left`
      (set `self.direction` "Up")
      (goto _label :!via `PlayFromStart`))))

(event `TurnLeft`
  (bind _returnvalue (`self.K2_GetActorRotation`))
  (set `self.rotate` true)
  (set `self.currentRotation` _returnvalue)
  (set `self.nextRotation` (`KismetMathLibrary.ComposeRotators` _returnvalue (struct :`Yaw` -90.0)))
  (switch `EDirection` (`self.direction`)
    (:`Up`
      (set `self.direction` "Left")
      (goto _label :!via `PlayFromStart`))
    (:`Right`
      (set `self.direction` "Up")
      (goto _label :!via `PlayFromStart`))
    (:`Down`
      (set `self.direction` "Right")
      (goto _label :!via `PlayFromStart`))
    (:`Left`
      (set `self.direction` "Down")
      (goto _label :!via `PlayFromStart`))))

(event `ResetPosition`
  (params (location :type "Vector Structure"))
  (set `self.died` false)
  (bind _asabp_character (cast `/Game/Asset/Character/Animation/ABP_Character` (`SkeletalMeshComponent.GetAnimInstance` (`self.Mesh`))))
  (set `/Game/Asset/Character/Animation/ABP_Character.died` false _asabp_character)
  (set `self.move` false)
  (set `self.location` (`self.spawnLocation`))
  (bind _output_get (set `self.direction` (`self.spawnDirection`)))
  (switch `EDirection` _output_get
    (:`Up`
      (set `self.rotation` (struct :`Pitch` -90.0)))
    (:`Right`
      (set `self.rotation` (struct)))
    (:`Down`
      (set `self.rotation` (struct :`Pitch` 90.0)))
    (:`Left`
      (set `self.rotation` (struct :`Pitch` 180.0))))
  (`self.K2_SetActorLocationAndRotation` location (`self.rotation`)))

(event `Die`
  (set `self.died` true)
  (`KismetSystemLibrary.Delay` 0.3)
  (bind _asabp_character (cast `/Game/Asset/Character/Animation/ABP_Character` (`SkeletalMeshComponent.GetAnimInstance` (`self.Mesh`))))
  (set `/Game/Asset/Character/Animation/ABP_Character.died` true _asabp_character))

(fn `UserConstructionScript`
  (`SceneComponent.K2_SetRelativeLocation` (`self.Mesh`) (0.0 0.0 0.0) false false)
  (`SceneComponent.K2_AddRelativeLocation` (`self.Mesh`) (`KismetMathLibrary.MakeVector` 0.0 0.0 (- 0.0 (`CapsuleComponent.GetScaledCapsuleHalfHeight` (`self.CapsuleComponent`)))) false false))